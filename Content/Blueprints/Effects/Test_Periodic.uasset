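; Test periodic effect that deals fixed Health damage to its target each period and prints a running tick count.
; On initialization it binds to the causer's player controller Attributes damage-caused event, then runs the first tick immediately; a non-player causer gets neither.
; That event handler adds the changed attribute's ModValue to the damage causer's Health, reacting to damage the instigator causes.
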(event `self.OnEffectPeriod`
  (bind _effectcauser (`self.EffectCauser`))
  (set `self.Counter` (+ (`self.Counter`) 1) :!label _label)
  (`KismetSystemLibrary.PrintString` (`KismetStringLibrary.BuildString_Int` "Effect Tick: " " " (`self.Counter`)))
  (`AREffectStatics.ApplyDamage` (`self.EffectTarget`) 4.0 "Health" _effectcauser _effectcauser (struct) false "/Script/Engine.DamageType"))

(event `self.OnEffectInitialized`
  (bind _asarcharacter (cast `ARCharacter` (`self.EffectCauser`)))
  (bind _asarplayercontroller (cast `ARPlayerController` (`Pawn.GetController` _asarcharacter)))
  (add `ARAttributeBaseComponent.OnInstigatorCausedDamage` (`ARPlayerController.Attributes` _asarplayercontroller) (delegate `OnConInstigatorCausedDamage_Event`))
  (goto _label))

(event `OnConInstigatorCausedDamage_Event`
  (params (AttributeChanged :type "AttributeChanged Structure"))
  (bind (_attribute _hitlocation _damagetarget _damagecauser) (break `AttributeChanged` AttributeChanged))
  (`KismetSystemLibrary.PrintString` "Effect Active")
  (`AREffectStatics.ChangeAttribute` _damagecauser (`self.EffectCauser`) (`.ModValue` (break `Attribute` _attribute)) "Health" "Attr_Add"))

(fn `UserConstructionScript`)