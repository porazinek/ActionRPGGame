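; Test effect field that deals radial damage to Health around its location on each field tick.
; Each tick applies full, falloff-free damage within the Collision sphere's radius, ignoring the field itself.
; On initialization it binds the field's begin-overlap event, which only prints the entering actor's name on the authority.
; A direct Collision overlap binding is left unconnected, and its handlers are empty.
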(event `self.OnFieldInitialized`
  (add `self.OnBeginFieldOverlap` (delegate `OnBeginFieldOverlap_Event`)))

(event `OnBeginFieldOverlap_Event` :!signature `self.OnBeginFieldOverlap`
  (params (OtherTags :type "ARFieldBase.FieldTags Structure") (OtherActor :type "Actor Object Reference") (OtherComp :type "PrimitiveComponent Object Reference") (bFromSweep :type Boolean) (SweepResult :type "EngineTypes.HitResult Structure (by ref)"))
  (`/Engine/EditorBlueprintResources/ActorMacros.Switch Has Authority`
    (:`Authority`
      (`KismetSystemLibrary.PrintString` (`KismetSystemLibrary.GetDisplayName` OtherActor)))))

(event `self.OnFieldTick`
  (bind _ignoreactors (`self.IgnoreActors`))
  (`KismetArrayLibrary.Array_Add` _ignoreactors self)
  (`AREffectStatics.ApplyRadialDamage` "Health" 3.0 (`self.K2_GetActorLocation` self) (`SphereComponent.SphereRadius` (`self.Collision`)) "/Script/Engine.DamageType" _ignoreactors self self true))

(event `self.Collision.OnComponentBeginOverlap`
  (params (OtherActor :type "Actor Object Reference") (OtherComp :type "PrimitiveComponent Object Reference") (OtherBodyIndex :type Integer) (bFromSweep :type Boolean) (SweepResult :type "EngineTypes.HitResult Structure (by ref)")))

(event `OnComponentBeginOverlap_Event`
  (params (OtherActor :type "Actor Object Reference") (OtherComp :type "PrimitiveComponent Object Reference") (OtherBodyIndex :type Integer) (bFromSweep :type Boolean) (SweepResult :type "EngineTypes.HitResult Structure (by ref)")))

(fn `UserConstructionScript`)