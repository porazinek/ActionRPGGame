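; BP_MovingMesh is a prototype sun and sky rig that is set up entirely in its construction script.
; Sun angle, rotation and Time values orient the actor and directional light and place a scaled sun mesh opposite the computed light vector.
; Dynamic materials tint the sun from the light or a custom color and pass sky color, sun color, light direction and brightness to a scalable, hideable skydome.
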(fn `UserConstructionScript`
  (bind _directionallight1 (`self.DirectionalLight1`))
  (bind _sunmeshscale (`self.SunMeshScale`))
  (bind _skydomescale (`self.SkyDomeScale`))
  (bind _skymaterial (`self.SkyMaterial`))
  (bind (_r _g _b) (`KismetMathLibrary.BreakColor` (`self.SunColor`)))
  (`SceneComponent.SetWorldScale3D` (`self.SkyDome`) (`KismetMathLibrary.MakeVector` _skydomescale _skydomescale _skydomescale))
  (`|ExecutionSequence`
    (:`then_0`
      (`LightComponent.SetIntensity` (`self.DirectionalLight1`) (`self.SunIntensity`))
      (`LightComponent.SetLightColor` (`self.DirectionalLight1`) (`self.SunLightColor`))
      (bind _returnvalue (`KismetMaterialLibrary.CreateDynamicMaterialInstance` "/Game/Blueprints/RandomPrototypes/M_SunMaterial_Master.M_SunMaterial_Master"))
      (if (not (`self.CustomSunColor`))
        (set `self.SunColor` (`KismetMathLibrary.Conv_ColorToLinearColor` (`LightComponentBase.LightColor` _directionallight1))))
      (set `self.SunMaterial` _returnvalue)
      (`MaterialInstanceDynamic.SetVectorParameterValue` (`self.SunMaterial`) "SunColor" (make `Object.LinearColor` _r _g _b (* (`LightComponentBase.Intensity` _directionallight1) (`self.ColorMultiplier`))))
      (`PrimitiveComponent.SetMaterial` (`self.StaticMesh1`) 0 (`self.SunMaterial`))
      (`self.SetActorRotation` (`KismetMathLibrary.MakeRot` (`self.SunRotation`) 0.0 (`self.SunAngle`)))
      (`SceneComponent.SetRelativeRotation` (`self.DirectionalLight1`) (`KismetMathLibrary.MakeRot` 0.0 (`self.Time`)) false)
      (`SceneComponent.SetWorldScale3D` (`self.StaticMesh1`) (`KismetMathLibrary.MakeVector` _sunmeshscale _sunmeshscale _sunmeshscale))
      (set `self.RotatorTest` (`KismetMathLibrary.MakeRot` (`self.SunAngle`) (`self.Time`) (`self.SunRotation`)))
      (set `self.XVectorTest` (`KismetMathLibrary.Conv_RotatorToVector` (`self.RotatorTest`)))
      (set `self.SunLocation` (* (`self.XVectorTest`) (* (`self.SunMeshDistance`) -1.0)))
      (`SceneComponent.SetRelativeLocation` (`self.StaticMesh1`) (`self.SunLocation`) false))
    (:`then_1`
      (bind _returnvalue_2 (`KismetMaterialLibrary.CreateDynamicMaterialInstance` "/Game/Blueprints/RandomPrototypes/M_Skydome.M_Skydome"))
      (set `self.SkyMaterial` _returnvalue_2)
      (`MaterialInstanceDynamic.SetVectorParameterValue` (`self.SkyMaterial`) "SkyColor" (`self.SkyColor`))
      (`MaterialInstanceDynamic.SetVectorParameterValue` (`self.SkyMaterial`) "LightDirection" (`KismetMathLibrary.Conv_VectorToLinearColor` (`KismetMathLibrary.MakeVector` (* (.x (`KismetMathLibrary.Conv_RotatorToVector` (`KismetMathLibrary.MakeRot` (`self.SunAngle`) (`self.Time`) (`self.SunRotation`)))) -10.0) (.y (`KismetMathLibrary.Conv_RotatorToVector` (`KismetMathLibrary.MakeRot` (`self.SunAngle`) (`self.Time`) (`self.SunRotation`)))) (* (.z (`KismetMathLibrary.Conv_RotatorToVector` (`KismetMathLibrary.MakeRot` (`self.SunAngle`) (`self.Time`) (`self.SunRotation`)))) -10.0))))
      (`MaterialInstanceDynamic.SetVectorParameterValue` _skymaterial "LightColor" (`self.SunColor`))
      (`MaterialInstanceDynamic.SetScalarParameterValue` _skymaterial "Brightness" (`self.RimeBrigthness`))
      (`PrimitiveComponent.SetMaterial` (`self.SkyDome`) 0 (`self.SkyMaterial`))
      (`SceneComponent.SetVisibility` (`self.SkyDome`) (`self.SkyVisible`) false))))