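; MyCharacter2 is a character Blueprint that acts as a test harness for its Equipment, Attributes and Abilities components.
; BeginPlay sets all three components to replicate.
; Tab flip-flops mouse cursor, click and hover events against look and move input, while Q adds two test weapons to the inventory and R adds a test ability.
; Disconnected leftover chains cover item swapping, action bar assignment and a delayed item add.
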(event `Key|Tab`
  (bind _returnvalue (`GameplayStatics.GetPlayerController` 0))
  (:`Pressed`
    (`/Engine/EditorBlueprintResources/StandardMacros.FlipFlop`
      (:`A`
        (set `PlayerController.bEnableClickEvents` false _returnvalue)
        (set `PlayerController.bEnableMouseOverEvents` false _returnvalue)
        (set `PlayerController.bShowMouseCursor` false _returnvalue)
        (`PlayerController.SetIgnoreLookInput` _returnvalue false)
        (`PlayerController.SetIgnoreMoveInput` _returnvalue false))
      (:`B`
        (set `PlayerController.bEnableClickEvents` true _returnvalue)
        (set `PlayerController.bEnableMouseOverEvents` true _returnvalue)
        (set `PlayerController.bShowMouseCursor` true _returnvalue)
        (`PlayerController.SetIgnoreLookInput` _returnvalue true)
        (`PlayerController.SetIgnoreMoveInput` _returnvalue true)))))

(event `self.ReceiveBeginPlay`
  (`ActorComponent.SetIsReplicated` (`self.Equipment`) true)
  (`ActorComponent.SetIsReplicated` (`self.Attributes`) true)
  (`ActorComponent.SetIsReplicated` (`self.Abilities`) true))

(event `Key|Q`
  (bind _equipment (`self.Equipment`))
  (:`Pressed`
    (`AREquipmentComponent.AddItemToInventory` _equipment (make `InventorySlot` "RedWeapon" "Item_Weapon" "Item_Chest"))
    (`AREquipmentComponent.AddItemToInventory` _equipment (make `InventorySlot` "TestWeapon" "Item_Weapon" "Item_Chest"))))

(event `Key|F`)

(event `Key|R`
  (:`Pressed`
    (`ARAbilityComponent.AddAbility` (`self.Abilities`) (make `AbilityInfo` "TestAbility" "/Game/Blueprints/Abilities/Test_Ability.Test_Ability_C"))))

(fn `UserConstructionScript`)