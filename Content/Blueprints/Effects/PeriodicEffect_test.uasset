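; PeriodicEffect_test is a test periodic effect that prints debug strings when attribute and damage events fire around its causer.
; On initialization it binds to attribute and point-attribute change events on the causer ARCharacter and its ARPlayerController, plus the controller's instigator-caused-damage event.
; The damage handler prints "Instigator Attack" and the others print "Causer Attack".
; The period event is empty, leaving a test print unconnected.
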(event `self.OnEffectPeriod`)

(event `self.OnEffectInitialized`
  (bind _asarcharacter (cast `ARCharacter` (`self.EffectCauser`)))
  (bind _attributes (`ARCharacter.Attributes` _asarcharacter))
  (add `ARAttributeBaseComponent.OnAttributeChanged` _attributes (delegate `OnAttributeChanged_Event`))
  (add `ARAttributeBaseComponent.OnPointAttributeChange` _attributes (delegate `OnPointAttributeChange_Event`))
  (bind _asarplayercontroller (cast `ARPlayerController` (`Pawn.GetController` _asarcharacter)))
  (bind _attributes_2 (`ARPlayerController.Attributes` _asarplayercontroller))
  (add `ARAttributeBaseComponent.OnInstigatorCausedDamage` _attributes_2 (delegate `OnInstigatorCausedDamage_Event`))
  (add `ARAttributeBaseComponent.OnAttributeChanged` _attributes_2 (delegate `OnConAttributeChanged_Event`))
  (add `ARAttributeBaseComponent.OnPointAttributeChange` _attributes_2 (delegate `OnConPointAttributeChange_Event`)))

(event `OnAttributeChanged_Event`
  (params (AttributeChanged :type "AttributeChanged Structure"))
  (`KismetSystemLibrary.PrintString` "Causer Attack"))

(event `OnPointAttributeChange_Event`
  (params (Attribute :type "Attribute Structure") (InstigatedBy :type "Actor Object Reference") (HitLocation :type "Object.Vector Structure") (FHitComponent :type "PrimitiveComponent Object Reference") (BoneName :type Name) (ShotFromDirection :type "Object.Vector Structure") (DamageType :type "DamageType Object Reference") (DamageCauser :type "Actor Object Reference"))
  (`KismetSystemLibrary.PrintString` "Causer Attack"))

(event `OnConAttributeChanged_Event`
  (params (AttributeChanged :type "AttributeChanged Structure"))
  (`KismetSystemLibrary.PrintString` "Causer Attack"))

(event `OnInstigatorCausedDamage_Event`
  (params (AttributeChanged :type "AttributeChanged Structure"))
  (`KismetSystemLibrary.PrintString` "Instigator Attack"))

(event `OnConPointAttributeChange_Event`
  (params (Attribute :type "Attribute Structure") (InstigatedBy :type "Actor Object Reference") (HitLocation :type "Object.Vector Structure") (FHitComponent :type "PrimitiveComponent Object Reference") (BoneName :type Name) (ShotFromDirection :type "Object.Vector Structure") (DamageType :type "DamageType Object Reference") (DamageCauser :type "Actor Object Reference"))
  (`KismetSystemLibrary.PrintString` "Causer Attack"))

(fn `UserConstructionScript`)