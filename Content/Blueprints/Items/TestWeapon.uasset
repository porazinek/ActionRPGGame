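; Test weapon Blueprint built on a replicated WeaponState action component with beam, trail-impact and targeting-decal cues, apparently a work in progress.
; Client action start binds WeaponState's cast and interval callbacks; interval, cast-start and server action-start events all run a left-hand weapon trace from the owner.
; Cast end stops the beam.
; Beam firing, damage draining and impact effects are disconnected, so traces apply nothing here, and ModifyDamageByAttribute is never called.
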(event `self.OnWeaponActive`
  (`ActorComponent.SetIsReplicated` (`self.ARTargetingDecal1`) false)
  (`ActorComponent.SetIsReplicated` (`self.ARBeamCue1`) true)
  (`ActorComponent.SetIsReplicated` (`self.WeaponState`) true))

(event `self.ClientOnActionStart`
  (bind _weaponstate (`self.WeaponState`))
  (`ActorComponent.SetIsReplicated` _weaponstate true)
  ;[1 1 1] Setup it in C++
  (set `ARActionStateComponent.Owner` (`self.ARCharacterOwner`) _weaponstate)
  (add `ARActionStateComponent.OnActionCastBegin` _weaponstate (delegate `OnActionCastBegin_Event`))
  (add `ARActionStateComponent.OnActionInterval` _weaponstate (delegate `OnActionInterval_Event`)))

(event `OnActionCastBegin_Event`
  (params (TagsOwnedByAction :type "GameplayTagContainer Structure (by ref)")))

(event `OnActionInterval_Event`
  (bind _archaracterowner (`self.ARCharacterOwner`))
  (bind _returnvalue (`Controller.CastToPlayerController` (`Pawn.GetController` _archaracterowner) :!label _label))
  (`ARTraceStatics.GetHitResult` 5000.0 "WeaponSocket" _archaracterowner false false "Trace_Weapon" "WeaponLeft"))

(event `self.OnCastStart`
  (goto _label))

(event `self.OnActionInterval`
  (goto _label))

(event `self.ServerOnActionStart`
  (goto _label))

(event `self.OnCastEnd`
  (set `ARBeamCue.IsFiring` false (`self.ARBeamCue1`)))

(event `self.OnActionEnd`)

(fn `ModifyDamageByAttribute`
  (params (DamageIn :type "Float (double-precision)"))
  (returns (ReturnValue :type "Float (double-precision)"))
  (return (+ DamageIn 5.0)))

(fn `UserConstructionScript`)