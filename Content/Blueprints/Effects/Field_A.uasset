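; Field_A is an effect field that can combine with other overlapping fields to form a new one.
; When an overlapping field has any of the required gameplay tags, it calls CombineFields to create a Field_C with a fixed duration.
; On received damage it runs the parent logic and prints the damage causer's name for debugging.
; The bound attribute damage handler is empty, and the particle collision binding is unwired.
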(event `self.OnFieldInitialized`
  (add `ARAttributeBaseComponent.OnAttributeDamage` (`self.Attributes`) (delegate `OnAttributeDamage_Event`)))

(event `OnAttributeDamage_Event`
  (params (AttributeChanged :type "AttributeChanged Structure") (DamageTag :type "GameplayTagContainer Structure")))

(event `self.OnReceiveFieldsOverlap`
  (params (OtherTags :type "ARFieldBase.FieldTags Structure") (OtherField :type "ARFieldBase Object Reference"))
  (if (`self.HasAnyMatchingGameplayTags` OtherField (`self.RequiredTags`) false)
    (`self.CombineFields` "/Game/Blueprints/Effects/Field_C.Field_C_C" 15.0 0.0 OtherField)))

(event `OnParticleCollide_Event`
  (params (EventName :type Name) (EmitterTime :type "Float (double-precision)") (ParticleTime :type Integer) (Location :type "Object.Vector Structure") (Velocity :type "Object.Vector Structure") (Direction :type "Object.Vector Structure") (Normal :type "Object.Vector Structure") (BoneName :type Name)))

(event `self.OnRecivedDamage`
  (params (AttributeChanged :type "AttributeChanged Structure") (Damage :type "ARDamageEvent Structure (by ref)") (DamageTag :type "GameplayTagContainer Structure"))
  (`parent.OnRecivedDamage` AttributeChanged Damage DamageTag)
  (`KismetSystemLibrary.PrintString` (`KismetSystemLibrary.GetDisplayName` (`.DamageCauser` (break `AttributeChanged` AttributeChanged)))))

(fn `UserConstructionScript`)