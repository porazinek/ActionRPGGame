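; Test feat effect that temporarily adds a flat damage bonus to the target character's right-hand weapon during each action.
; On initialization it listens to the ARCharacter's Equipment for the active right weapon, then binds to that weapon's WeaponState cast events.
; Pre-cast stores the original damage and raises it, and cast end restores it.
; Debug prints mark weapon assignment and use.
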(event `self.OnEffectInitialized`
  (bind _asarcharacter (cast `ARCharacter` (`self.EffectTarget`)))
  (add `AREquipmentComponent.OnRightWeaponActive` (`ARCharacter.Equipment` _asarcharacter) (delegate `OnRightWeaponActive_Event`)))

(event `OnRightWeaponActive_Event`
  (params (Weapon :type "ARWeapon Object Reference"))
  (bind _weaponstate (`ARWeapon.WeaponState` Weapon))
  (set `self.CurrentWeapon` Weapon)
  (add `ARActionStateComponent.OnActionPreCast` _weaponstate (delegate `OnActionPreCast_Event`))
  (add `ARActionStateComponent.OnActionCastEnd` _weaponstate (delegate `OnActionCastEnd_Event`))
  (`KismetSystemLibrary.PrintString` "Weapon Assigned"))

(event `OnActionPreCast_Event`
  (bind _damage (`ARWeapon.Damage` (`self.CurrentWeapon`)))
  (`KismetSystemLibrary.PrintString` "Weapon Used")
  (set `self.OriginalDamage` _damage)
  (set `ARWeapon.Damage` (+ _damage 10.0) (`self.CurrentWeapon`)))

(event `OnActionCastEnd_Event`
  (set `ARWeapon.Damage` (`self.OriginalDamage`) (`self.CurrentWeapon`)))