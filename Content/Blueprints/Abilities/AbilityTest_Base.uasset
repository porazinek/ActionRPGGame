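; AbilityTest_Base is a test ability Blueprint that reports the lifecycle of its action state.
; On action start it binds handlers to the ActionState's cast begin, cast end, cooldown begin and cooldown end events.
; Each handler prints a debug message, and BeginPlay sets the ActionState to replicate.
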(event `self.OnActionStart`
  (bind _actionstate (`self.ActionState`))
  (add `ARActionStateComponent.OnActionCastBegin` _actionstate (delegate `OnActionCastBegin_Event`))
  (add `ARActionStateComponent.OnActionCastEnd` _actionstate (delegate `OnActionCastEnd_Event`))
  (add `ARActionStateComponent.OnCooldownBegin` _actionstate (delegate `OnCooldownBegin_Event`))
  (add `ARActionStateComponent.OnCooldownEnded` _actionstate (delegate `OnCooldownEnded_Event`)))

(event `self.ReceiveBeginPlay`
  (`ActorComponent.SetIsReplicated` (`self.ActionState`) true))

(event `OnActionCastBegin_Event`
  (`KismetSystemLibrary.PrintString` "Ability casting started"))

(event `OnActionCastEnd_Event`
  (`KismetSystemLibrary.PrintString` "Ability Casted"))

(event `OnCooldownBegin_Event`
  (`KismetSystemLibrary.PrintString` "Cooldown Started"))

(event `OnCooldownEnded_Event`
  (`KismetSystemLibrary.PrintString` "Cooldown ended"))

(fn `UserConstructionScript`)