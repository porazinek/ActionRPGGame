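; Feat effect that modifies damage the character who caused it receives.
; On initialization it casts that causer to ARCharacter and binds to the incoming-damage event on its Attributes component.
; The handler subtracts a flat amount from each incoming modifier value and submits it as final damage, without clamping.
; A temporary right-weapon damage boost with restore on cast end remains as disconnected logic and empty events.
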(event `self.OnEffectInitialized`
  (bind _asarcharacter (cast `ARCharacter` (`self.EffectCausedBy`)))
  (bind _attributes (`ARCharacter.Attributes` _asarcharacter))
  (set `self.Attributecomp` _attributes)
  (add `ARAttributeBaseComponent.OnIncomingDamage` _attributes (delegate `OnIncomingDamage_Event`)))

(event `OnIncomingDamage_Event`
  (params (DamageTags :type "GameplayTagContainer Structure (by ref)") (Attribute :type "Attribute Structure (by ref)"))
  (bind (_attributename _modvalue _operationtype) (break `Attribute` Attribute))
  (`ARAttributeBaseComponent.SetFinalDmage` (`self.Attributecomp`) (make `Attribute` _attributename (- _modvalue 5.0) _operationtype)))

(event `OnRightWeaponActive_Event`
  (params (Weapon :type "ARWeapon Object Reference")))

(event `OnActionPreCast_Event`)

(event `OnActionCastEnd_Event`
  ;[1 1 1] Restore original damage to weapon, after player finish using it to void stacking indefinte damage
)