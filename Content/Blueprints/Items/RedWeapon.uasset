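; RedWeapon is a weapon item Blueprint that spawns a timed, ticking Field_A where the owner's weapon trace hits.
; When the action starts on the server, it binds to WeaponState's cast-begin and interval events.
; Both events share one path: a long-range hit trace feeding SpawnField, with the owner as instigator.
; Projectile, periodic-effect, effect-cue and debug-print nodes remain disconnected and never run.
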(event `self.ServerOnActionStart`
  (bind _weaponstate (`self.WeaponState`))
  (add `ARActionStateComponent.OnActionCastBegin` _weaponstate (delegate `OnActionCastBegin_Event`))
  (add `ARActionStateComponent.OnActionInterval` _weaponstate (delegate `OnActionInterval_Event`)))

(event `OnActionCastBegin_Event`
  (params (TagsOwnedByAction :type "GameplayTagContainer Structure (by ref)"))
  (bind _returnvalue (`ARTraceStatics.GetHitResult` 5000.0 "None" (`self.WeaponOwner`) false false "Trace_Weapon" :!label _label))
  (`AREffectStatics.SpawnField` "/Game/Blueprints/Effects/Field_A.Field_A_C" (`self.WeaponOwner`) _returnvalue 10.0 1.0))

(event `OnActionInterval_Event`
  (goto _label))

(fn `UserConstructionScript`)